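; Player controller for a Dungeon Keeper style prototype that lets the player hover and paint-select blocks with a visible mouse cursor.
; Each tick it traces from the camera along the deprojected mouse direction, with debug drawing, and sends mouse-over and mouse-out calls to Block_BP actors as the hit changes.
; Pressing the left button sets the brush to the inverse of the hovered block's selection, then applies that state to every block hovered while held.
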(event `self.ReceiveBeginPlay`
  (set `self.bShowMouseCursor` true))

(event `self.ReceiveTick`
  (params (DeltaSeconds :type "Float (single-precision)"))
  (bind _on_hit_actor (`self.on hit actor`))
  (bind _returnvalue (`PlayerCameraManager.GetCameraLocation` (`GameplayStatics.GetPlayerCameraManager` 0)))
  (bind (_outhit _returnvalue_2) (`KismetSystemLibrary.LineTraceSingle` :`Start` _returnvalue :`End` (+ _returnvalue (* (`.WorldDirection` (`self.DeprojectMousePositionToWorld`)) 9999.0)) :`TraceChannel` "TraceTypeQuery1" :`DrawDebugType` "ForDuration" :`DrawTime` 1.0))
  (if _returnvalue_2
    (`/Engine/EditorBlueprintResources/StandardMacros.IsValid` _on_hit_actor
      (:`Is Valid`
        (if (!= _on_hit_actor (`.HitActor` (`GameplayStatics.BreakHitResult` _outhit)))
          (bind _asblock_bp (cast `/Game/proto_dugeon_keeper/Block_BP` (`self.on hit actor`))
            (:`then`
              (`/Game/proto_dugeon_keeper/Block_BP.mouse out` _asblock_bp))
            (:`CastFailed`
              _))))
      (:`Is Not Valid`
        _))
    (bind _output_get (set `self.on hit actor` (`.HitActor` (`GameplayStatics.BreakHitResult` _outhit))))
    (bind _asblock_bp_2 (cast `/Game/proto_dugeon_keeper/Block_BP` _output_get))
    (`/Game/proto_dugeon_keeper/Block_BP.mose over` _asblock_bp_2)
    (if (`self.is mouse down`)
      (set `/Game/proto_dugeon_keeper/Block_BP.is selected` (`self.selection brush`) _asblock_bp_2))))

(event `Key|LeftMouseButton`
  (params (Key :type "Key Structure"))
  (bind _on_hit_actor (`self.on hit actor`))
  (:`Pressed`
    (set `self.is mouse down` true)
    (`/Engine/EditorBlueprintResources/StandardMacros.IsValid` _on_hit_actor
      (:`Is Valid`
        (bind _asblock_bp (cast `/Game/proto_dugeon_keeper/Block_BP` _on_hit_actor))
        (set `self.selection brush` (not (`/Game/proto_dugeon_keeper/Block_BP.is selected` _asblock_bp))))))
  (:`Released`
    (set `self.is mouse down` false)))

(fn `UserConstructionScript`)