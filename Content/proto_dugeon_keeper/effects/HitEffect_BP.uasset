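; HitEffect_BP is a short-lived billboard visual effect, apparently spawned to mark a hit.
; On BeginPlay it sets a one-second lifespan, picks a random direction and switches the billboard to absolute scale.
; Each tick it drifts along that direction at its Velocity and halves the billboard's world scale, so the shrink depends on frame rate rather than delta time.
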(event `self.ReceiveBeginPlay`
  (`self.SetLifeSpan` 1.0)
  (set `self.translation vector` (`KismetMathLibrary.RandomUnitVector`))
  (set `SceneComponent.bAbsoluteScale` true (`self.Billboard`)))

(event `self.ReceiveTick`
  (params (DeltaSeconds :type "Float (single-precision)"))
  (bind _billboard (`self.Billboard`))
  (`self.K2_AddActorLocalOffset` (* (* (`self.translation vector`) (`self.velocity`)) DeltaSeconds))
  (`SceneComponent.SetWorldScale3D` _billboard (* (`SceneComponent.K2_GetComponentScale` _billboard) 0.5)))

(fn `UserConstructionScript`)