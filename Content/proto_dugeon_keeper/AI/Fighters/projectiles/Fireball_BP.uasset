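; Fireball projectile for AI fighters that damages characters on the opposing side in the dungeon keeper prototype.
; On spawn it launches along Direction at the set Velocity through ProjectileMovement, with a short lifespan.
; Sphere overlaps filter for AI characters, using IsPlayersFireball and interface checks to hit only player enemies or only player allies.
; A valid hit spawns HitEffect_BP at the target, applies Damage and destroys the fireball.
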(event `self.ReceiveBeginPlay`
  (`self.SetLifeSpan` 5.0)
  (set `MovementComponent.Velocity` (* (`self.direction`) (`self.velocity`)) (`self.ProjectileMovement`)))

(event `self.Sphere.OnComponentBeginOverlap`
  (params (OverlappedComponent :type "PrimitiveComponent Object Reference") (OtherActor :type "Actor Object Reference") (OtherComp :type "PrimitiveComponent Object Reference") (OtherBodyIndex :type Integer) (bFromSweep :type Boolean) (SweepResult :type "HitResult Structure (by ref)"))
  (bind _output_get (set `self.the other actor` OtherActor))
  (if (`KismetSystemLibrary.DoesImplementInterface` _output_get "/Game/proto_dugeon_keeper/AI/peon/IAICharacter.IAICharacter_C")
    (if (`self.is players fireball?`)
      (if (`KismetSystemLibrary.DoesImplementInterface` (`self.the other actor`) "/Game/proto_dugeon_keeper/AI/Fighters/Enemy_AI/IPlayerEnemy.IPlayerEnemy_C")
        (`|ExecutionSequence` :!label _label
          (:`then_0`
            (`|SpawnActorFromClass` "/Game/proto_dugeon_keeper/effects/HitEffect_BP.HitEffect_BP_C" (`KismetMathLibrary.MakeTransform` (`self.K2_GetActorLocation` (`self.the other actor`))) "Undefined" "OverrideRootScale" null null))
          (:`then_1`
            (`GameplayStatics.ApplyDamage` (`self.the other actor`) (`self.damage`) null (`self.Instigator`)))
          (:`then_2`
            (`self.K2_DestroyActor`))))
      (elif (`KismetSystemLibrary.DoesImplementInterface` (`self.the other actor`) "/Game/proto_dugeon_keeper/AI/Fighters/Monsters_AI/IPlayerAlly.IPlayerAlly_C")
        (goto _label)))))

(fn `UserConstructionScript`)