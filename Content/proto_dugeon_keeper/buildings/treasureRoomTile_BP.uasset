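; Treasure room tile Blueprint for a dungeon keeper prototype that stores gold up to a maximum capacity.
; Every Tick uniformly scales the SceneScale component by the ratio of stashed gold to capacity, showing how full the tile is.
; Query functions report whether free space remains, true whenever stashed gold differs from capacity, and return current and total gold as room stats.
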(event `self.ReceiveTick`
  (params (DeltaSeconds :type "Float (single-precision)"))
  (bind _returnvalue (/ (`KismetMathLibrary.Conv_IntToDouble` (`self.gold stashed`)) (`KismetMathLibrary.Conv_IntToDouble` (`self.max capacity`))))
  (`SceneComponent.SetRelativeScale3D` (`self.Scene scale`) (`KismetMathLibrary.MakeVector` _returnvalue _returnvalue _returnvalue)))

(fn `get room stats`
  (returns (current :type Integer) (total :type Integer) (`value name` :type String))
  (return (`self.gold stashed`) (`self.max capacity`) "gold"))

(fn `has free space for gold`
  (returns (`has free space?` :type Boolean))
  (return (not (== (`self.max capacity`) (`self.gold stashed`)))))

(fn `UserConstructionScript`)