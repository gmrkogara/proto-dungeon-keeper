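; Block_BP is a destructible block in a dungeon keeper prototype that leaves a gold pile when destroyed.
; On BeginPlay it rolls a small random hit point count, and each damage event removes one point regardless of amount.
; At zero it spawns GoldPile_BP at its location and destroys itself.
; Mouse-over and mouse-out events swap the mesh material for hover feedback, with the restored material depending on IsSelected.
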(event `self.ReceiveAnyDamage`
  (params (Damage :type "Float (single-precision)") (DamageType :type "DamageType Object Reference") (InstigatedBy :type "Controller Object Reference") (DamageCauser :type "Actor Object Reference"))
  (`KismetSystemLibrary.PrintString` "block got dmg")
  (bind _result (`/Engine/EditorBlueprintResources/StandardMacros.DecrementInt` (`self.hitpoints`))
    (:`  `
      (if (== _result 0)
        (`|ExecutionSequence`
          (:`then_0`
            (`|SpawnActorFromClass` "/Game/proto_dugeon_keeper/goldPile_BP.goldPile_BP_C" (`KismetMathLibrary.MakeTransform` (`self.K2_GetActorLocation`)) "Undefined" "OverrideRootScale" null null))
          (:`then_1`
            (`self.K2_DestroyActor`)))))))

(event `self.ReceiveBeginPlay`
  (set `self.hitpoints` (`KismetMathLibrary.RandomIntegerInRange` 2 3)))

(event `mose over`
  (`PrimitiveComponent.SetMaterial` (`self.StaticMesh`) 0 "/Game/proto_dugeon_keeper/NewMaterial_Inst.NewMaterial_Inst"))

(event `mouse out`
  (if (`self.is selected`)
    (`PrimitiveComponent.SetMaterial` (`self.StaticMesh`) 0 "/Game/StarterContent/Materials/M_Wood_Oak.M_Wood_Oak")
    (else
      (`PrimitiveComponent.SetMaterial` (`self.StaticMesh`) 0 "/Engine/BasicShapes/BasicShapeMaterial.BasicShapeMaterial"))))

(fn `UserConstructionScript`)