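; Enemy spawner building for the dungeon keeper prototype that keeps a capped population of living enemies once activated.
; An actor implementing IPlayerAlly entering ActivationBox activates the house permanently, destroying the box.
; A delay-throttled Tick prunes invalid enemies, then, below the cap and after a random wait, spawns a class from a random data table row.
; Each spawn is tracked, gets a default controller and runs the configured behavior tree.
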(event `self.ReceiveTick`
  (params (DeltaSeconds :type "Float (single-precision)"))
  (bind (_returnvalue_x _returnvalue_y _returnvalue_z) (`KismetMathLibrary.BreakVector` (`self.K2_GetActorLocation`)))
  (`KismetSystemLibrary.Delay` 0.2)
  (`|ExecutionSequence`
    (:`then_0`
      (`self.validate living enemies`))
    (:`then_1`
      (if (and (`self.is active`) (< (`KismetArrayLibrary.Array_Length` (`self.living enemies`)) (`self.max enemies`)))
        (`KismetSystemLibrary.Delay` (`KismetMathLibrary.RandomFloatInRange` 3.0 10.0))
        (bind _outrownames (`DataTableFunctionLibrary.GetDataTableRowNames` (`self.spawn from table`)))
        (bind _returnvalue (`|GetDataTableRow` (`self.spawn from table`) (`|GetArrayItem` _outrownames (`KismetMathLibrary.RandomInteger` (`KismetArrayLibrary.Array_Length` _outrownames))))
          (:`then`
            (bind _returnvalue_2 (`|SpawnActorFromClass` (`.actorclass_28_70889B9C4F94F544413895B603D727FD` (break `/Game/proto_dugeon_keeper/AI/MonsterProperties` _returnvalue)) (`KismetMathLibrary.MakeTransform` (`KismetMathLibrary.MakeVector` _returnvalue_x _returnvalue_y (+ _returnvalue_z 100.0))) "Undefined" "OverrideRootScale" null null))
            (bind _output_get (set `self.last actor` _returnvalue_2))
            (`KismetArrayLibrary.Array_Add` (`self.living enemies`) _output_get)
            (`Pawn.SpawnDefaultController` (`Actor.Instigator` _output_get))
            (`AIController.RunBehaviorTree` (`AIBlueprintHelperLibrary.GetAIController` (`self.last actor`)) (`self.behaviour tree`))))))))

(event `validate living enemies`
  (for _array_element (`self.living enemies`)
    (if (not (`KismetSystemLibrary.IsValid` _array_element))
      (`KismetArrayLibrary.Array_RemoveItem` (`self.living enemies`) _array_element))))

(event `self.Activate`
  (params (`By player?` :type Boolean))
  ;[1 1 1] activation
)

(event `self.activation box.OnComponentBeginOverlap`
  (params (OverlappedComponent :type "PrimitiveComponent Object Reference") (OtherActor :type "Actor Object Reference") (OtherComp :type "PrimitiveComponent Object Reference") (OtherBodyIndex :type Integer) (bFromSweep :type Boolean) (SweepResult :type "HitResult Structure (by ref)"))
  ;[1 1 1] activation
  (bind _output_get (set `self.is active` (`KismetSystemLibrary.DoesImplementInterface` OtherActor "/Game/proto_dugeon_keeper/AI/Fighters/Monsters_AI/IPlayerAlly.IPlayerAlly_C")))
  (if _output_get
    (`ActorComponent.K2_DestroyComponent` (`self.activation box`))
    (`KismetSystemLibrary.PrintString` "enemies house overlap")))

(fn `UserConstructionScript`
  (`parent.UserConstructionScript`))