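; Level grid for the dungeon keeper prototype that builds a tiled floor and randomly fills it with blocks.
; The construction script lays scaled Floor instances at each cell center of an X by Y grid macro.
; On BeginPlay, BrushBox teleports to each cell, skipping any that overlap a Spacer_BP.
; Remaining cells spawn Block_BP when a random float exceeds BlocksDensity, so higher values yield fewer blocks.
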(event `self.ReceiveBeginPlay`
  (bind _scale (`self.scale`))
  (bind (_current_point _total_points _0_1_phase _poly_center) (`/Engine/ArtTools/RenderToTexture/Macros/RenderToTextureMacros.2D Grid Execution Macro` (* (`self.scale`) (`self.sector size`)) (0.0 0.0 0.0) (`self.x`) (`self.y`))
    (:`Per Poly Execution`
      (set `self.poly center` _poly_center)
      (set `self.draw cube` true)
      (`|ExecutionSequence`
        (:`then_0`
          (`SceneComponent.K2_SetWorldLocation` (`self.Brush Box`) (`self.poly center`) false true)
          (for _array_element (`PrimitiveComponent.GetOverlappingActors` (`self.Brush Box`) null)
            (if (== (`GameplayStatics.GetObjectClass` _array_element) "/Game/proto_dugeon_keeper/Spacer_BP.Spacer_BP_C")
              (set `self.draw cube` false))))
        (:`then_1`
          (if (`self.draw cube`)
            (if (> (`KismetMathLibrary.RandomFloat`) (`self.blocks density`))
              (`|SpawnActorFromClass` "/Game/proto_dugeon_keeper/buildings/Block_BP.Block_BP_C" (`KismetMathLibrary.MakeTransform` (`self.poly center`) (struct) (`KismetMathLibrary.MakeVector` _scale _scale _scale)) "Undefined" "OverrideRootScale" null null))))))))

(fn `UserConstructionScript`
  (locals (`loop poly center` :type "Vector Structure" :default (0.0 0.0 0.0)))
  (bind _scale (`self.scale`))
  (bind _scale_2 (`self.scale`))
  (`|ExecutionSequence`
    (:`then_0`
      (bind (_current_point _total_points _0_1_phase _poly_center) (`/Engine/ArtTools/RenderToTexture/Macros/RenderToTextureMacros.2D Grid Execution Macro` (* (`self.sector size`) (`self.scale`)) (0.0 0.0 0.0) (`self.x`) (`self.y`))
        (:`Per Poly Execution`
          (set `local.loop poly center` _poly_center)
          (`InstancedStaticMeshComponent.AddInstance` (`self.floor`) (`KismetMathLibrary.MakeTransform` (`local.loop poly center`) (struct) (`KismetMathLibrary.MakeVector` _scale _scale _scale))))))
    (:`then_1`
      (`SceneComponent.SetWorldScale3D` (`self.Brush Box`) (`KismetMathLibrary.MakeVector` _scale_2 _scale_2 _scale_2)))))