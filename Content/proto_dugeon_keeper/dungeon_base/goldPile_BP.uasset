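; Gold pile pickup actor for the dungeon keeper prototype, built from five cube meshes.
; MarkedasPickedUp sets the IsPickedUp flag and hides all five cubes rather than destroying the actor.
; Get Money returns a fresh random gold amount within a fixed range on each call, and Is it picked up? exposes the flag to callers.
; It has no overlap or tick logic, so pickup is triggered externally.
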(event `/Game/proto_dugeon_keeper/IDugeonItem.Marked as picked up`
  (set `self.is picked up` true)
  (for _array_element (`|MakeArray` (`self.Cube1`) (`self.Cube2`) (`self.Cube3`) (`self.Cube4`) (`self.Cube`))
    (`SceneComponent.SetHiddenInGame` _array_element true false)))

(fn `Get Money`
  (returns (money :type Integer))
  (return (`KismetMathLibrary.RandomIntegerInRange` 20 50)))

(fn `Is it picked up?`
  (returns (`Is It ?` :type Boolean))
  (return (`self.is picked up`)))

(fn `UserConstructionScript`)