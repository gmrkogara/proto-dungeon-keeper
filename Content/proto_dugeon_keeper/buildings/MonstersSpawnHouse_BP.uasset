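; Monster spawn house building for the dungeon keeper prototype, which spawns AI monsters above itself once activated.
; While active, Tick uses a Delay as a random-interval timer, rebuilding the eligible monster list and spawning one random type from it.
; A data table drives eligibility: each type's target population grows with game-state TotalSpent relative to its UnlockAt, capped at ten.
; The bound middle-mouse handler is empty, its debug refresh left disconnected.
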(event `self.ReceiveBeginPlay`
  (bind _asdk_game_state (cast `/Game/proto_dugeon_keeper/player/dk_gameState` (`GameplayStatics.GetGameState`)))
  (set `self.dk game state` _asdk_game_state)
  (bind _asdk_player_controller_bp (cast `/Game/proto_dugeon_keeper/player/dk_player_controller_BP` (`GameplayStatics.GetPlayerController` 0)))
  (add `/Game/proto_dugeon_keeper/player/dk_player_controller_BP.MMB Down` _asdk_player_controller_bp (delegate `on mmb down`)))

(event `on mmb down`
  (params (`is down` :type Boolean)))

(event `self.ReceiveTick`
  (params (DeltaSeconds :type "Float (single-precision)"))
  (bind (_returnvalue_x _returnvalue_y _returnvalue_z) (`KismetMathLibrary.BreakVector` (`self.K2_GetActorLocation`)))
  (bind _monsters_to_spawn (`self.monsters to spawn`))
  (if (`self.is active`)
    (`KismetSystemLibrary.Delay` (`KismetMathLibrary.RandomFloatInRange` 0.5 3.0))
    (`|ExecutionSequence`
      (:`then_0`
        (`self.get monsters to spawn count`))
      (:`then_1`
        (if (> (`KismetArrayLibrary.Array_Length` _monsters_to_spawn) 0)
          (`|SpawnActorFromClass` "/Game/proto_dugeon_keeper/AI/AI_character_spawn_BP.AI_character_spawn_BP_C" (`KismetMathLibrary.MakeTransform` (`KismetMathLibrary.MakeVector` _returnvalue_x _returnvalue_y (+ _returnvalue_z 100.0))) "Undefined" "OverrideRootScale" null (`|GetArrayItem` _monsters_to_spawn (`KismetMathLibrary.RandomInteger` (`KismetArrayLibrary.Array_Length` _monsters_to_spawn))) null))))))

(event `/Game/proto_dugeon_keeper/IDungeonBuilding.Activate`
  (params (`By player?` :type Boolean))
  (set `self.is active` true)
  (`KismetSystemLibrary.PrintString` "house activated"))

(event `get monsters to spawn count`
  (`KismetArrayLibrary.Array_Clear` (`self.monsters to spawn`))
  (bind _outrownames (`DataTableFunctionLibrary.GetDataTableRowNames` "/Game/proto_dugeon_keeper/AI/MonstersDataTable.MonstersDataTable"))
  (for _array_element _outrownames
    (`KismetSystemLibrary.PrintString` (`KismetStringLibrary.Conv_NameToString` _array_element))
    (bind _returnvalue (`|GetDataTableRow` "/Game/proto_dugeon_keeper/AI/MonstersDataTable.MonstersDataTable" _array_element)
      (:`then`
        (bind (_monstertype _unlockat _life _walkspeed _hungdywalkspeed _damageperattack _attackspeed _attackrange _food _actorclass) (break `/Game/proto_dugeon_keeper/AI/MonsterProperties` _returnvalue))
        (if (`|EnumInequality` _monstertype "NewEnumerator5")
          (`|ExecutionSequence`
            (:`then_0`
              (bind _outactors (`GameplayStatics.GetAllActorsOfClass` _actorclass))
              (bind _count (`/Game/proto_dugeon_keeper/dk_global_functions.get number of monsters of type` _outactors _monstertype))
              (bind _output_get (set `self.count of current monster type` _count))
              (`KismetSystemLibrary.PrintString` (`KismetStringLibrary.Conv_IntToString` _output_get)))
            (:`then_1`
              (if (< (`self.count of current monster type`) 10)
                (if (> (`KismetMathLibrary.Clamp` (- (`.ReturnValue` (`KismetMathLibrary.FMod` (`KismetMathLibrary.Conv_IntToDouble` (`/Game/proto_dugeon_keeper/player/dk_gameState.total spent` (`self.dk game state`))) (`KismetMathLibrary.Conv_IntToDouble` _unlockat))) (`self.count of current monster type`)) 0 10) 0)
                  (`KismetArrayLibrary.Array_Add` (`self.monsters to spawn`) _monstertype))))))))))

(fn `UserConstructionScript`)