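; DungeonFloor_BP is a dungeon floor tile that can be claimed by the player or converted into a treasure room or chicken farm.
; Conversion sets the tile type and swaps the ChildActorComponent to the matching room actor, with random yaw for treasure.
; Each state change stores its material in MouseOutMaterial, so the MouseOver highlight can revert to the current look on MouseOut.
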(event `/Game/proto_dugeon_keeper/IMouseOverOut.Mouse over`
  (`PrimitiveComponent.SetMaterial` (`self.Cube`) 0 "/Game/proto_dugeon_keeper/materials/tile_selection_Material_Inst.tile_selection_Material_Inst"))

(event `convert to treasure tile`
  (set `self.tile type` "NewEnumerator1")
  (`ChildActorComponent.SetChildActorClass` (`self.ChildActorComponent`) "/Game/proto_dugeon_keeper/buildings/treasureRoomTile_BP.treasureRoomTile_BP_C")
  (bind _output_get (set `self.mouse out material` "/Game/proto_dugeon_keeper/materials/gold_tile_material_Inst.gold_tile_material_Inst"))
  (`PrimitiveComponent.SetMaterial` (`self.Cube`) 0 _output_get)
  (`SceneComponent.K2_SetRelativeRotation` (`self.ChildActorComponent`) (`KismetMathLibrary.MakeRotator` 0.0 0.0 (`KismetMathLibrary.RandomFloatInRange` 0.0 90.0)) false false))

(event `/Game/proto_dugeon_keeper/IMouseOverOut.Mouse out`
  (`PrimitiveComponent.SetMaterial` (`self.Cube`) 0 (`self.mouse out material`)))

(event `mark as claimed by player`
  (set `self.is claimed by player?` true)
  (bind _output_get (set `self.mouse out material` "/Game/proto_dugeon_keeper/materials/player_claimed_tile_material_Inst.player_claimed_tile_material_Inst"))
  (`PrimitiveComponent.SetMaterial` (`self.Cube`) 0 _output_get))

(event `convert to chicken farm`
  (set `self.tile type` "NewEnumerator2")
  (`ChildActorComponent.SetChildActorClass` (`self.ChildActorComponent`) "/Game/proto_dugeon_keeper/buildings/FarmRoomTile_BP.FarmRoomTile_BP_C")
  (bind _output_get (set `self.mouse out material` "/Game/proto_dugeon_keeper/materials/chickenFarm_tile_material_Inst.chickenFarm_tile_material_Inst"))
  (`PrimitiveComponent.SetMaterial` (`self.Cube`) 0 _output_get))

(fn `UserConstructionScript`)