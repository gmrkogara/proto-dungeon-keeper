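; Lair room tile for the dungeon keeper prototype, serving as a bed that a single monster can claim.
; Claiming stores the monster reference, with no check for an existing owner.
; Every tick, after the parent update, the billboard shows only while that reference is valid.
; Room stats report the tile as one "Monster lair" slot, occupied when the monster is valid.
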(event `self.ReceiveTick`
  (params (DeltaSeconds :type "Float (single-precision)"))
  (`parent.ReceiveTick` DeltaSeconds)
  (`SceneComponent.SetHiddenInGame` (`self.Billboard`) (not (`KismetSystemLibrary.IsValid` (`self.monster `))) false))

(fn `claim monster lair `
  (params (`monster owning the bed` :type "Actor Object Reference"))
  (set `self.monster ` `monster owning the bed`))

(fn `get room stats`
  (returns (current :type Integer) (total :type Integer) (`value name` :type String))
  (locals (`the string to show` :type String))
  (`|ExecutionSequence`
    (:`then_0`
      (if true
        _))
    (:`then_1`
      (return (select `bool` (`KismetSystemLibrary.IsValid` (`self.monster `)) :`true` 1) 1 "Monster lair"))))

(fn `UserConstructionScript`
  (`parent.UserConstructionScript`))