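; Placeable one-shot spawner that creates a monster of the chosen MonsterType in the dungeon keeper prototype.
; The construction script looks up that type's MonstersDataTable row and shows its icon on the billboard.
; On BeginPlay it reads the row, spawns the row's actor class at its location and calls SpawnDefaultController on that actor's instigator.
; It then passes the monster properties to the spawned actor by interface message and destroys itself.
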(event `self.ReceiveBeginPlay`
  (bind (_monster_properties_monstertype _monster_properties_unlockat _monster_properties_life _monster_properties_walkspeed _monster_properties_damageperattack _monster_properties_attackspeed _monster_properties_attackrange _monster_properties_food _monster_properties_actorclass) (break `/Game/proto_dugeon_keeper/AI/MonsterProperties` (`self.monster properties`)))
  (`|ExecutionSequence`
    (:`then_0`
      (bind _returnvalue (`|GetDataTableRow` "/Game/proto_dugeon_keeper/AI/Fighters/MonstersDataTable.MonstersDataTable" (`KismetStringLibrary.Conv_StringToName` (`|GetEnumeratorNameAsString` (`self.monster type`))))
        (:`then`
          (set `self.monster properties` _returnvalue))))
    (:`then_1`
      (bind _returnvalue_2 (`|SpawnActorFromClass` _monster_properties_actorclass (`KismetMathLibrary.MakeTransform` (`self.K2_GetActorLocation`)) "Undefined" "OverrideRootScale" null null))
      (bind _output_get (set `self.actor` _returnvalue_2))
      (`Pawn.SpawnDefaultController` (`Actor.Instigator` _output_get)))
    (:`then_2`
      (message `/Game/proto_dugeon_keeper/AI/peon/IAICharacter.set monster properties` (`self.actor`) (`self.monster properties`)))
    (:`then_3`
      (`self.K2_DestroyActor`))))

(fn `UserConstructionScript`
  (bind _returnvalue (`|GetDataTableRow` "/Game/proto_dugeon_keeper/AI/Fighters/MonstersDataTable.MonstersDataTable" (`KismetStringLibrary.Conv_StringToName` (`|GetEnumeratorNameAsString` (`self.monster type`))))
    (:`then`
      (bind _astexture_2d (cast `Texture2D` (`.icon_31_B1FC8D0A4D47FDF3E34DD8A40A84F25A` (break `/Game/proto_dugeon_keeper/AI/MonsterProperties` _returnvalue)))
        (:`then`
          (`BillboardComponent.SetSprite` (`self.Billboard`) _astexture_2d))
        (:`CastFailed`
          (`KismetSystemLibrary.PrintString` "text ture cast failed"))))
    (:`RowNotFound`
      (`KismetSystemLibrary.PrintString` "row not found"))))