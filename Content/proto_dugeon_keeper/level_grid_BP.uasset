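; Level grid actor for a dungeon keeper prototype that builds a tiled floor and scatters blocks over it.
; A shared 2D grid macro walks X by Y cells at the scaled sector size.
; The construction script adds a floor instance at each cell center.
; BeginPlay spawns a Block_BP on cells where a random roll exceeds BlocksDensity, so higher density values yield fewer blocks.
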(event `self.ReceiveBeginPlay`
  (bind _scale (`self.scale`))
  (bind (_current_point _total_points _0_1_phase _poly_center) (`/Engine/ArtTools/RenderToTexture/Macros/RenderToTextureMacros.2D Grid Execution Macro` (* (`self.scale`) (`self.sector size`)) (0.0 0.0 0.0) (`self.x`) (`self.y`))
    (:`Per Poly Execution`
      (if (> (`KismetMathLibrary.RandomFloat`) (`self.blocks density`))
        (`|SpawnActorFromClass` "/Game/proto_dugeon_keeper/Block_BP.Block_BP_C" (`KismetMathLibrary.MakeTransform` _poly_center (struct) (`KismetMathLibrary.MakeVector` _scale _scale _scale)) "Undefined" "OverrideRootScale" null null)))))

(fn `UserConstructionScript`
  (locals (`loop poly center` :type "Vector Structure" :default (0.0 0.0 0.0)))
  (bind _scale (`self.scale`))
  (bind (_current_point _total_points _0_1_phase _poly_center) (`/Engine/ArtTools/RenderToTexture/Macros/RenderToTextureMacros.2D Grid Execution Macro` (* (`self.sector size`) (`self.scale`)) (0.0 0.0 0.0) (`self.x`) (`self.y`))
    (:`Per Poly Execution`
      (set `local.loop poly center` _poly_center)
      (`InstancedStaticMeshComponent.AddInstance` (`self.floor`) (`KismetMathLibrary.MakeTransform` (`local.loop poly center`) (struct) (`KismetMathLibrary.MakeVector` _scale _scale _scale))))))