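; MonstersHouseSpawner_BP is a one-shot placement actor that puts a monster spawn house onto a dungeon floor tile.
; On BeginPlay it takes the first overlapping DungeonFloor_BP and moves itself to that tile's location.
; It then sets the floor's ChildActorComponent class to MonstersSpawnHouse_BP and destroys itself.
; If the cast to the floor fails, it prints an error message.
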(event `self.ReceiveBeginPlay`
  (bind _asdungeon_floor_bp (cast `/Game/proto_dugeon_keeper/dungeon_base/DungeonFloor_BP` (`|GetArrayItem` (`self.GetOverlappingActors` self "/Game/proto_dugeon_keeper/dungeon_base/DungeonFloor_BP.DungeonFloor_BP_C")))
    (:`then`
      (bind _output_get (set `self.floor bp` _asdungeon_floor_bp))
      (`|ExecutionSequence`
        (:`then_0`
          (`self.K2_SetActorLocation` (`self.K2_GetActorLocation` (`self.floor bp`))))
        (:`then_1`
          (`ChildActorComponent.SetChildActorClass` (`/Game/proto_dugeon_keeper/dungeon_base/DungeonFloor_BP.ChildActorComponent` _output_get) "/Game/proto_dugeon_keeper/buildings/MonstersSpawnHouse_BP.MonstersSpawnHouse_BP_C"))
        (:`then_2`
          (`self.K2_DestroyActor`))))
    (:`CastFailed`
      (`KismetSystemLibrary.PrintString` (`KismetStringLibrary.JoinStringArray` (`|MakeArray` (`KismetSystemLibrary.GetDisplayName` self) "failed to cast"))))))

(fn `UserConstructionScript`)