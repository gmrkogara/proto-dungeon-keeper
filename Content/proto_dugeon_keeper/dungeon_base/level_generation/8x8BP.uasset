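; Procedural box block for dungeon level generation that subdivides into smaller actors on mouse-over.
; The construction script builds the mesh from CubeSize; MouseOver spawns a Slices-by-Slices grid of DividedActorClass pieces and hides it.
; A bound FocusIsOut event destroys the pieces and unhides the mesh, but IsDivided stays true and this Blueprint's FocusIsOut call is unwired.
; DivideBlock and DivideBlock0 are alternative division functions, uncalled here.
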(event `/Game/proto_dugeon_keeper/IMouseOverOut.Mouse over`
  (bind (_box_extent_x _box_extent_y) (`KismetMathLibrary.BreakVector` (`self.box extent`)))
  (bind _box_extent_x_2 (`KismetMathLibrary.BreakVector` (`self.box extent`)))
  (`KismetSystemLibrary.PrintString` (`KismetSystemLibrary.GetDisplayName` self))
  (`KismetArrayLibrary.Array_Clear` (`self.pieces`))
  (if (and (`self.can divide`) (== (`self.is divided`) false))
    (set `self.box extent` (`.BoxExtent` (`KismetSystemLibrary.GetComponentBounds` (`self.ProceduralMesh`))))
    (`|ExecutionSequence`
      (:`then_0`
        (bind (_current_point _total_points _0_1_phase _poly_center _x_row _y_row) (`/Engine/ArtTools/RenderToTexture/Macros/RenderToTextureMacros.2D Grid Execution Macro` _box_extent_x_2 (0.0 0.0 0.0) (`self.slices`) (`self.slices`))
          (:`Per Poly Execution`
            (bind _returnvalue (`|SpawnActorFromClass` (`self.divided actor class`) (`KismetMathLibrary.MakeTransform` (+ (* (`KismetMathLibrary.MakeVector` (`KismetMathLibrary.Conv_IntToDouble` _x_row) (`KismetMathLibrary.Conv_IntToDouble` _y_row) 1.0) (/ (* (`KismetMathLibrary.MakeVector` _box_extent_x _box_extent_y) 2.0) (`KismetMathLibrary.Conv_IntToDouble` (`self.slices`)))) (`self.K2_GetActorLocation`))) "Undefined" "OverrideRootScale" self null))
            (set `self.current piece` _returnvalue)
            (add `self.focus is out` (delegate `on focus is out`))
            (`KismetArrayLibrary.Array_Add` (`self.pieces`) _returnvalue)
            (`SceneComponent.SetHiddenInGame` (`self.ProceduralMesh`) true false))))
      (:`then_1`
        (set `self.is divided` true)))))

(event `on focus is out`
  (`self.roll back division`))

(event `/Game/proto_dugeon_keeper/IMouseOverOut.Mouse out`)

(fn `divide block`
  (locals (`box extent` :type "Vector Structure" :default (0.0 0.0 0.0)))
  (if (and (`self.can divide`) (== (`self.is divided`) false))
    (set `local.box extent` (`.BoxExtent` (`KismetSystemLibrary.GetComponentBounds` null)))
    (for _array_element (`|MakeArray` (`KismetMathLibrary.MakeVector2D` 1.0) (`KismetMathLibrary.MakeVector2D` 0.0 1.0) (`KismetMathLibrary.MakeVector2D` 1.0 1.0) (`KismetMathLibrary.MakeVector2D` 0.0 0.0))
      (`|SpawnActorFromClass` (`self.divided actor class`) (`KismetMathLibrary.MakeTransform` (+ (* (`KismetMathLibrary.MakeVector` (`KismetMathLibrary.BreakVector2D` _array_element) (`.Y` (`KismetMathLibrary.BreakVector2D` _array_element)) 1.0) (`local.box extent`)) (`self.K2_GetActorLocation`))) "Undefined" "OverrideRootScale" null null)
      (`SceneComponent.SetHiddenInGame` (`self.ProceduralMesh`) true false))
    (set `self.is divided` true)))

(fn `divide block_0`
  (locals (`box extent` :type "Vector Structure" :default (0.0 0.0 0.0)) (`current piece` :type "Actor Object Reference"))
  (bind (_box_extent_x _box_extent_y) (`KismetMathLibrary.BreakVector` (`local.box extent`)))
  (bind _box_extent_x_2 (`KismetMathLibrary.BreakVector` (`local.box extent`)))
  (`KismetArrayLibrary.Array_Clear` (`self.pieces`))
  (if (and (`self.can divide`) (== (`self.is divided`) false))
    (set `local.box extent` (`.BoxExtent` (`KismetSystemLibrary.GetComponentBounds` null)))
    (`|ExecutionSequence`
      (:`then_0`
        (bind (_current_point _total_points _0_1_phase _poly_center _x_row _y_row) (`/Engine/ArtTools/RenderToTexture/Macros/RenderToTextureMacros.2D Grid Execution Macro` _box_extent_x_2 (0.0 0.0 0.0) (`self.slices`) (`self.slices`))
          (:`Per Poly Execution`
            (bind _returnvalue (`|SpawnActorFromClass` (`self.divided actor class`) (`KismetMathLibrary.MakeTransform` (+ (* (`KismetMathLibrary.MakeVector` (`KismetMathLibrary.Conv_IntToDouble` _x_row) (`KismetMathLibrary.Conv_IntToDouble` _y_row) 1.0) (/ (* (`KismetMathLibrary.MakeVector` _box_extent_x _box_extent_y) 2.0) (`KismetMathLibrary.Conv_IntToDouble` (`self.slices`)))) (`self.K2_GetActorLocation`))) "Undefined" "OverrideRootScale" self null))
            (set `local.current piece` _returnvalue)
            (`KismetArrayLibrary.Array_Add` (`self.pieces`) _returnvalue)
            (`SceneComponent.SetHiddenInGame` (`self.ProceduralMesh`) true false))))
      (:`then_1`
        (set `self.is divided` true)))))

(fn `roll back division`
  (for _array_element (`self.pieces`)
    (`self.K2_DestroyActor` _array_element))
  (`KismetArrayLibrary.Array_Clear` (`self.pieces`))
  (`SceneComponent.SetHiddenInGame` (`self.ProceduralMesh`) false false))

(fn `UserConstructionScript`
  (bind _proceduralmesh (`self.ProceduralMesh`))
  (bind _returnvalue (* (`self.cube size`) 100.0))
  (bind (_vertices _triangles _normals _uvs _tangents) (`KismetProceduralMeshLibrary.GenerateBoxMesh` (`KismetMathLibrary.MakeVector` _returnvalue _returnvalue 100.0)))
  (`ProceduralMeshComponent.CreateMeshSection_LinearColor` :`self` _proceduralmesh :`Vertices` _vertices :`Triangles` _triangles :`Normals` _normals :`UV0` _uvs :`Tangents` _tangents)
  (`PrimitiveComponent.SetMaterial` _proceduralmesh 0 (`self.material`)))