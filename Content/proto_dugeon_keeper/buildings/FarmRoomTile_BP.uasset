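; Farm room tile for a dungeon keeper prototype that produces food in the form of chickens.
; Tick grows the food value up to capacity and spawns a chicken above the tile whenever its whole hundreds exceed the living chicken count.
; Each chicken gets a default controller and a death callback that removes it and subtracts its value from the food.
; GetRoomStats reports current and maximum food.
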(event `self.ReceiveTick`
  (params (DeltaSeconds :type "Float (single-precision)"))
  (bind _output_get (set `self.current value` (`KismetMathLibrary.FClamp` (+ (`self.current value`) (* DeltaSeconds (`self.diff per sec`))) 0.0 (`self.max capacity`))))
  (if (> (`.ReturnValue` (`KismetMathLibrary.FMod` _output_get 100.0)) (`KismetArrayLibrary.Array_Length` (`self.chickens`)))
    (`self.spawn chicken`)))

(event `spawn chicken`
  (bind (_returnvalue_x _returnvalue_y _returnvalue_z) (`KismetMathLibrary.BreakVector` (`self.K2_GetActorLocation`)))
  (bind _returnvalue (`|SpawnActorFromClass` "/Game/proto_dugeon_keeper/AI/FarmChicken/FarmChickenCharacter.FarmChickenCharacter_C" (`KismetMathLibrary.MakeTransform` (`KismetMathLibrary.MakeVector` _returnvalue_x _returnvalue_y (+ _returnvalue_z 100.0))) "Undefined" "OverrideRootScale" self null))
  (bind _output_get (set `self.spawned chicken` _returnvalue :!label _label))
  (`/Engine/EditorBlueprintResources/StandardMacros.IsValid` _output_get
    (:`Is Valid`
      (`Pawn.SpawnDefaultController` _output_get)
      (`KismetArrayLibrary.Array_Add` (`self.chickens`) (`self.spawned chicken`))
      (add `/Game/proto_dugeon_keeper/AI/FarmChicken/FarmChickenCharacter.chicken died` (`self.spawned chicken`) (delegate `on chicken died`)))
    (:`Is Not Valid`
      (`KismetSystemLibrary.Delay` 0.2)
      (goto _label))))

(event `on chicken died`
  (params (`the chicken` :type "Actor Object Reference"))
  (`KismetArrayLibrary.Array_RemoveItem` (`self.chickens`) `the chicken`)
  (set `self.current value` (- (`self.current value`) (`self.chicken value`))))

(fn `get room stats`
  (returns (current :type Integer) (total :type Integer) (`value name` :type String))
  (return (`KismetMathLibrary.FTrunc` (`self.current value`)) (`KismetMathLibrary.FTrunc` (`self.max capacity`)) "Food"))

(fn `UserConstructionScript`)