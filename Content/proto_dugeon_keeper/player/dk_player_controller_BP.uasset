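; Player controller for a dungeon keeper prototype that turns mouse input into digging, peon spawning and treasure room building.
; Each tick a camera-to-cursor trace tracks the hovered actor, sending mouse over/out messages and showing a treasure room widget at the cursor over treasure tiles.
; A controller mode routes left clicks to drag-brush dig selection, paid peon spawning or floor-to-treasure conversion; right click resets to block selection.
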(event `self.ReceiveBeginPlay`
  (set `self.bShowMouseCursor` true)
  (bind _asdk_game_state (cast `/Game/proto_dugeon_keeper/player/dk_gameState` (`GameplayStatics.GetGameState`)))
  (set `self.dk game state` _asdk_game_state)
  (bind _returnvalue (`|CreateWidget` "/Game/proto_dugeon_keeper/player/treasureRoom_Widget.treasureRoom_Widget_C"))
  (set `self.treasure room widget` _returnvalue))

(event `self.ReceiveTick`
  (params (DeltaSeconds :type "Float (single-precision)"))
  (switch `/Game/proto_dugeon_keeper/player/dk_controller_mode` (`self.controller mode`)
    (:`NewEnumerator0`
      _)
    (:`NewEnumerator1`
      _)
    (:`NewEnumerator2`
      _))
  (`self.select tile`))

(event `select tile`
  (bind _on_hit_actor (`self.on hit actor`))
  (bind _treasure_room_widget (`self.treasure room widget`))
  (bind _visible_widget (`self.visible widget`))
  (bind _returnvalue (`PlayerCameraManager.GetCameraLocation` (`GameplayStatics.GetPlayerCameraManager` 0)))
  (bind (_outhit _returnvalue_2) (`KismetSystemLibrary.LineTraceSingle` :`Start` _returnvalue :`End` (+ _returnvalue (* (`.WorldDirection` (`self.DeprojectMousePositionToWorld`)) 9999.0)) :`TraceChannel` "TraceTypeQuery1" :`DrawDebugType` "ForOneFrame" :`DrawTime` 1.0))
  (if _returnvalue_2
    (`/Engine/EditorBlueprintResources/StandardMacros.IsValid` _on_hit_actor
      (:`Is Valid`
        (if (!= _on_hit_actor (`.HitActor` (`GameplayStatics.BreakHitResult` _outhit)))
          (message `/Game/proto_dugeon_keeper/IMouseOverOut.Mouse out` (`self.on hit actor`))
          (`|ExecutionSequence`
            (:`then_0`
              (`/Engine/EditorBlueprintResources/StandardMacros.IsValid` _visible_widget
                (:`Is Valid`
                  (if (`Widget.IsInViewport` _visible_widget)
                    (`Widget.RemoveFromParent` _visible_widget)))))
            (:`then_1`
              (set `self.on hit actor` (`.HitActor` (`GameplayStatics.BreakHitResult` _outhit)) :!label _label)
              (switch `/Game/proto_dugeon_keeper/player/dk_controller_mode` (`self.controller mode`)
                (:`NewEnumerator0`
                  (`|ExecutionSequence`
                    (:`then_0`
                      (bind _asdungeon_block_bp (cast `/Game/proto_dugeon_keeper/dungeon_base/DungeonBlock_BP` (`self.on hit actor`)))
                      (message `/Game/proto_dugeon_keeper/IMouseOverOut.Mouse over` _asdungeon_block_bp)
                      (if (`self.is mouse down`)
                        (`/Game/proto_dugeon_keeper/dungeon_base/DungeonBlock_BP.mark as selected for dig` _asdungeon_block_bp (`self.selection brush`))))
                    (:`then_1`
                      (bind _asdungeon_floor_bp (cast `/Game/proto_dugeon_keeper/dungeon_base/DungeonFloor_BP` (`self.on hit actor`)))
                      (bind _astreasure_room_tile_bp (cast `/Game/proto_dugeon_keeper/buildings/treasureRoomTile_BP` (`ChildActorComponent.ChildActor` (`/Game/proto_dugeon_keeper/dungeon_base/DungeonFloor_BP.ChildActorComponent` _asdungeon_floor_bp))))
                      (set `/Game/proto_dugeon_keeper/player/treasureRoom_Widget.treasure room actor` _astreasure_room_tile_bp (`self.treasure room widget`))
                      (if (not (`Widget.IsInViewport` _treasure_room_widget))
                        (`UserWidget.AddToViewport` _treasure_room_widget 2))
                      (bind (_success _x _y) (`LowEntryExtendedStandardLibrary.GetMousePosition`))
                      (`UserWidget.SetPositionInViewport` _treasure_room_widget (`KismetMathLibrary.MakeVector2D` (`KismetMathLibrary.Conv_IntToDouble` _x) (`KismetMathLibrary.Conv_IntToDouble` _y)) true)
                      (set `self.visible widget` (`self.treasure room widget`)))))
                (:`NewEnumerator1`
                  (message `/Game/proto_dugeon_keeper/IMouseOverOut.Mouse over` (`self.on hit actor`) :!label _label_2)
                  (switch `/Game/proto_dugeon_keeper/player/dk_controller_mode` (`self.controller mode`)))
                (:`NewEnumerator2`
                  (goto _label_2)))))
          (else
            (goto _label))))
      (:`Is Not Valid`
        (goto _label)))))

(event `LMB select block for dig`
  (bind _on_hit_actor (`self.on hit actor`))
  (if (`self.is mouse down`)
    (`/Engine/EditorBlueprintResources/StandardMacros.IsValid` _on_hit_actor
      (:`Is Valid`
        (bind _asdungeon_block_bp (cast `/Game/proto_dugeon_keeper/dungeon_base/DungeonBlock_BP` _on_hit_actor))
        (set `self.selection brush` (not (`/Game/proto_dugeon_keeper/dungeon_base/DungeonBlock_BP.is selected` _asdungeon_block_bp)))))))

(event `LMB spawn peon`
  (bind _on_hit_actor (`self.on hit actor`))
  (bind (_returnvalue_x _returnvalue_y _returnvalue_z) (`KismetMathLibrary.BreakVector` (`self.K2_GetActorLocation` _on_hit_actor)))
  (if (`self.is mouse down`)
    (if (not (`self.lmb action done`))
      (if (>= (`/Game/proto_dugeon_keeper/player/dk_gameState.money` (`self.dk game state`)) (`self.peon price`))
        (`/Engine/EditorBlueprintResources/StandardMacros.IsValid` _on_hit_actor
          (:`Is Valid`
            (bind _returnvalue (`|SpawnActorFromClass` "/Game/proto_dugeon_keeper/AI/peon/PeonAICharacter.PeonAICharacter_C" (`KismetMathLibrary.MakeTransform` (`KismetMathLibrary.MakeVector` _returnvalue_x _returnvalue_y (+ _returnvalue_z 100.0))) "Undefined" "OverrideRootScale" null null))
            (`Pawn.SpawnDefaultController` _returnvalue)
            (set `self.lmb action done` true)
            (set `/Game/proto_dugeon_keeper/player/dk_gameState.money` (- (`/Game/proto_dugeon_keeper/player/dk_gameState.money` (`self.dk game state`)) (`self.peon price`)) (`self.dk game state`))))
        (else
          (`KismetSystemLibrary.PrintString` "not enough money to buy peon")
          (set `self.lmb action done` true))))))

(event `Key|LeftMouseButton`
  (params (Key :type "Key Structure"))
  (:`Pressed`
    (set `self.is mouse down` true)
    (switch `/Game/proto_dugeon_keeper/player/dk_controller_mode` (`self.controller mode`) :!label _label_3
      (:`NewEnumerator0`
        (`self.LMB select block for dig`))
      (:`NewEnumerator1`
        (`self.LMB spawn peon`))
      (:`NewEnumerator2`
        (`self.LMB build tresure tile`))))
  (:`Released`
    (set `self.lmb action done` false)
    (set `self.is mouse down` false)
    (goto _label_3)))

(event `Key|RightMouseButton`
  (params (Key :type "Key Structure"))
  (:`Pressed`
    (set `self.controller mode` "NewEnumerator0")))

(event `LMB build tresure tile`
  (`KismetSystemLibrary.PrintString` "build treasure room")
  (if (`self.is mouse down`)
    (if (not (`self.lmb action done`))
      (`/Engine/EditorBlueprintResources/StandardMacros.IsValid` (`self.on hit actor`)
        (:`Is Valid`
          (bind _asdungeon_floor_bp (cast `/Game/proto_dugeon_keeper/dungeon_base/DungeonFloor_BP` (`self.on hit actor`)))
          (`/Game/proto_dugeon_keeper/dungeon_base/DungeonFloor_BP.convert to treasure tile` _asdungeon_floor_bp)
          (set `self.lmb action done` true))))))

(fn `UserConstructionScript`)