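; Diggable dungeon wall block for a dungeon-keeper prototype that yields gold and becomes floor when destroyed.
; Each damage event spawns a gold pile at the damage causer and decrements randomized hitpoints; at zero, it spawns a floor tile and larger pile, then destroys itself.
; Dig selection switches the nav modifier between null and obstacle areas, while mouse events swap materials for hover and selection feedback.
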(event `self.ReceiveBeginPlay`
  (set `self.hitpoints` (`KismetMathLibrary.RandomIntegerInRange` 2 3)))

(event `self.ReceiveAnyDamage`
  (params (Damage :type "Float (single-precision)") (DamageType :type "DamageType Object Reference") (InstigatedBy :type "Controller Object Reference") (DamageCauser :type "Actor Object Reference"))
  (`|ExecutionSequence`
    (:`then_0`
      (`|SpawnActorFromClass` "/Game/proto_dugeon_keeper/dungeon_base/goldPile_BP.goldPile_BP_C" (`KismetMathLibrary.MakeTransform` (`self.K2_GetActorLocation` DamageCauser)) "Undefined" "OverrideRootScale" null (* (`KismetMathLibrary.RandomIntegerInRange` 5 30) (`self.gold multiplier`)) null)
      (`GameplayStatics.PlaySound2D` "/Game/proto_dugeon_keeper/sounds/shovel.shovel" 1.0 1.0 0.0 null null))
    (:`then_1`
      (bind _result (`/Engine/EditorBlueprintResources/StandardMacros.DecrementInt` (`self.hitpoints`))
        (:`  `
          (if (== _result 0)
            (`|ExecutionSequence`
              (:`then_0`
                (`|SpawnActorFromClass` "/Game/proto_dugeon_keeper/dungeon_base/DungeonFloor_BP.DungeonFloor_BP_C" (`self.GetTransform`) "Undefined" "OverrideRootScale" null null))
              (:`then_1`
                (`|SpawnActorFromClass` "/Game/proto_dugeon_keeper/dungeon_base/goldPile_BP.goldPile_BP_C" (`KismetMathLibrary.MakeTransform` (`self.K2_GetActorLocation`)) "Undefined" "OverrideRootScale" null (* (`KismetMathLibrary.RandomIntegerInRange` 25 75) (`self.gold multiplier`)) null))
              (:`then_2`
                (`self.K2_DestroyActor`)))))))))

(event `/Game/proto_dugeon_keeper/IMouseOverOut.Mouse over`
  (`PrimitiveComponent.SetMaterial` (`self.StaticMesh`) 0 "/Game/proto_dugeon_keeper/materials/blocks/tile_selection_Material_Inst.tile_selection_Material_Inst"))

(event `mark as selected for dig`
  (params (`true?` :type Boolean))
  (bind _output_get (set `self.is selected` `true?`))
  (if _output_get
    (`NavModifierComponent.SetAreaClass` (`self.NavModifier`) "/Script/NavigationSystem.NavArea_Obstacle")
    (else
      (`NavModifierComponent.SetAreaClass` (`self.NavModifier`) "/Script/NavigationSystem.NavArea_Null"))))

(event `/Game/proto_dugeon_keeper/IMouseOverOut.Mouse out`
  (if (`self.is selected`)
    (`PrimitiveComponent.SetMaterial` (`self.StaticMesh`) 0 "/Game/proto_dugeon_keeper/materials/blocks/selected-top-texture_block_mat_Inst.selected-top-texture_block_mat_Inst")
    (else
      (`PrimitiveComponent.SetMaterial` (`self.StaticMesh`) 0 "/Game/proto_dugeon_keeper/materials/blocks/top-texture-block_Mat_Inst.top-texture-block_Mat_Inst"))))

(fn `UserConstructionScript`)